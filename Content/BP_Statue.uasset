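; BP_Statue is a statue actor that shatters into Chaos debris when hit hard enough.
; A hit above an impulse threshold hides the static mesh once, stops its physics, then loads the statue Geometry Collection and applies external strain to break it.
; Each break event moves that piece to the Debris collision profile and calls GeometryCollectionBroken.
; The any-damage binding leads to an empty handler.
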(event OnChaosBreakEvent(GeometryCollection)
  (params (BreakEvent :type Chaos%20Break%20Event%20Structure%20%28by%20ref%29))
  (Class|GeometryCollectionComponent|SetPerParticleCollisionProfileName (Variables|Default|GetGeometryCollection) (Utilities|Array|MakeArray (.index BreakEvent)) "Debris")
  (Class|BreakableTarget|GeometryCollectionBroken (Variables|Default|GetBreak%20Event)))

(event Custom|CustomEvent
  (params (DamagedActor :type Actor%20Object%20Reference) (Damage :type Float%20%28single-precision%29) (DamageType :type Damage%20Type%20Object%20Reference) (InstigatedBy :type Controller%20Object%20Reference) (DamageCauser :type Actor%20Object%20Reference)))

(event EventBeginPlay
  (EventDispatchers|BindEventtoOnTakeAnyDamage (delegate Custom|CustomEvent))
  (Class|GeometryCollectionComponent|SetNotifyBreaks (Variables|Default|GetGeometryCollection) true))

(event Collision|EventHit
  (params (MyComp :type Primitive%20Component%20Object%20Reference) (Other :type Actor%20Object%20Reference) (OtherComp :type Primitive%20Component%20Object%20Reference) (bSelfMoved :type Boolean) (HitLocation :type Vector :default "0, 0, 0") (HitNormal :type Vector :default "0, 0, 0") (NormalImpulse :type Vector :default "0, 0, 0") (Hit :type Hit%20Result%20Structure%20%28by%20ref%29))
  (if (> (Math|Vector|VectorLength NormalImpulse) 1.5e+03)
    (Utilities|FlowControl|DoOnce false
      (:Completed
        (Rendering|SetVisibility (Variables|Default|GetStaticMesh) false false)
        (Class|GeometryCollectionComponent|SetRestCollection (Variables|Default|GetGeometryCollection) "/Game/GC_SM_Statue.GC_SM_Statue" true)
        (Class|GeometryCollectionComponent|ApplyExternalStrain (Variables|Default|GetGeometryCollection) 0 (Transformation|GetActorLocation) 0.0 0 1.0 5e+05)
        (Physics|SetSimulatePhysics (Variables|Default|GetStaticMesh) false)))))

(fn ConstructionScript)