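; Rifle pickup that attaches a hitscan weapon to the character who collects it and handles what its shots do on impact.
; On pickup, it attaches the HitscanWeapon, sets the rifle flag on the first-person AnimBP and binds the weapon's impact event.
; Each impact applies point damage with a linear damage type and triggers a short-lived FS_MasterField at the hit position for a directional physics-field push.
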(event OnPickUp(TP_PickUp)
  (params (PickUpCharacter :type Physics%20Character%20Object%20Reference))
  (bind _returnvalue (Class|PhysicsWeaponComponent|AttachWeapon (Variables|Default|GetHitscanWeapon) PickUpCharacter))
  (if _returnvalue
    (bind _asfirst_person_anim_bp (Utilities|Casting|CastToFirstPerson_AnimBP (Components|SkeletalMesh|GetAnimInstance (Variables|/Script/Physics.PhysicsCharacter|GetMesh1P PickUpCharacter))))
    (Variables|/Game/FirstPersonArms/Animations/FirstPerson_AnimBP.FirstPerson_AnimBP_C|SetHasRifle _asfirst_person_anim_bp true)
    (EventDispatchers|AssignOnHitscanImpact (Variables|Default|GetHitscanWeapon) (delegate Custom|onHitscanImpact_Event))))

(event Custom|onHitscanImpact_Event
  (params (impactedActor :type Actor%20Object%20Reference) (impactPosition :type Vector) (impactDirection :type Vector))
  (CallFunction|CEApplyDamage impactedActor impactDirection)
  (bind _returnvalue (Game|SpawnActorfromClass "/Engine/EditorResources/FieldNodes/FS_MasterField.FS_MasterField_C" (Math|Conversions|ToTransform(Vector) impactPosition) "Undefined" "MultiplyWithRoot" 0 0))
  (Variables|/Engine/EditorResources/FieldNodes/FS_MasterField.FS_MasterField_C|SetActivationType _returnvalue "NewEnumerator2")
  (Actor|SetLifeSpan _returnvalue 0.1)
  (Variables|/Engine/EditorResources/FieldNodes/FS_MasterField.FS_MasterField_C|SetDirectionalMagnitude _returnvalue 1e+04)
  (Default|CETrigger _returnvalue))

(event Custom|CE_ApplyDamage
  (params (DamagedActor :type Actor%20Object%20Reference) (HitFromDirection :type Vector%20%28by%20ref%29))
  (Game|Damage|ApplyPointDamage DamagedActor 5e+01 HitFromDirection (Variables|Default|GetHit%20Info) (Variables|Default|GetEvent%20Instigator) self "/Game/BP_DamageTypeLineal.BP_DamageTypeLineal_C"))

(fn ConstructionScript)